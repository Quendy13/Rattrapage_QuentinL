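; BP_Door is a puzzle door that opens once it has received a required number of Interact events.
; Each Interact increments a key counter; when it exactly equals the requirement, the Cube loses collision and is hidden.
; If the timer flag is set, a delay then restores the Cube's collision and visibility, closing the door without resetting the counter.
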(event `self.ReceiveTick`
  (params (DeltaSeconds :type "Float (single-precision)")))

(event `/Game/Interfaces/BPI_Interact.Interact`
  (bind _cube (`self.Cube`))
  (bind _cube_2 (`self.Cube`))
  (`/Engine/EditorBlueprintResources/StandardMacros.IncrementInt` (`self.nbKeys`)
    (:`  `
      (if (== (`self.nbKeys`) (`self.nbKeysRequirement`))
        (`|ExecutionSequence`
          (:`then_0`
            (`PrimitiveComponent.SetCollisionEnabled` _cube_2 "NoCollision"))
          (:`then_1`
            (`SceneComponent.SetVisibility` _cube_2 false false))
          (:`then_2`
            (if (`self.bIsTimer`)
              (`KismetSystemLibrary.Delay` (`self.Duration`))
              (`|ExecutionSequence`
                (:`then_0`
                  (`PrimitiveComponent.SetCollisionEnabled` _cube "QueryAndPhysics"))
                (:`then_1`
                  (`SceneComponent.SetVisibility` _cube true false))))))))))

(fn `UserConstructionScript`)