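; Spike trap that starts hidden and harmless, then activates on a delay after something overlaps its detection volume.
; Detection overlap waits two seconds, shows the spike with collision and sets an active flag, then reverts after five more seconds.
; While active, a top-down character entering the damage volume takes damage, and player character 0 is launched horizontally against its navigation movement velocity.
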(event `self.ReceiveBeginPlay`
  (bind _spike1 (`self.Spike1`))
  (`PrimitiveComponent.SetCollisionEnabled` _spike1 "NoCollision")
  (`SceneComponent.SetVisibility` _spike1 false false))

(event `self.DetectionCollision.OnComponentBeginOverlap`
  (params (OverlappedComponent :type "PrimitiveComponent Object Reference") (OtherActor :type "Actor Object Reference") (OtherComp :type "PrimitiveComponent Object Reference") (OtherBodyIndex :type Integer) (bFromSweep :type Boolean) (SweepResult :type "HitResult Structure (by ref)"))
  (bind _spike1 (`self.Spike1`))
  (bind _spike1_2 (`self.Spike1`))
  (`KismetSystemLibrary.Delay` 2.0)
  (`|ExecutionSequence`
    (:`then_0`
      (set `self.bIsActivated` true))
    (:`then_1`
      (`PrimitiveComponent.SetCollisionEnabled` _spike1 "QueryAndPhysics"))
    (:`then_2`
      (`SceneComponent.SetVisibility` _spike1 true false))
    (:`then_3`
      (`KismetSystemLibrary.Delay` 5.0)
      (`|ExecutionSequence`
        (:`then_0`
          (set `self.bIsActivated` false))
        (:`then_1`
          (`PrimitiveComponent.SetCollisionEnabled` _spike1_2 "NoCollision"))
        (:`then_2`
          (`SceneComponent.SetVisibility` _spike1_2 false false))))))

(event `self.DamageCollision.OnComponentBeginOverlap`
  (params (OverlappedComponent :type "PrimitiveComponent Object Reference") (OtherActor :type "Actor Object Reference") (OtherComp :type "PrimitiveComponent Object Reference") (OtherBodyIndex :type Integer) (bFromSweep :type Boolean) (SweepResult :type "HitResult Structure (by ref)"))
  (bind _asbp_top_down_character (cast `/Game/Blueprints/Character/BP_TopDownCharacter` OtherActor))
  (if (`self.bIsActivated`)
    (`GameplayStatics.ApplyDamage` _asbp_top_down_character 1.0)
    (bind _asbp_top_down_character_2 (cast `/Game/Blueprints/Character/BP_TopDownCharacter` (`GameplayStatics.GetPlayerCharacter` 0))
      (:`then`
        (bind (_returnvalue_x _returnvalue_y) (`KismetMathLibrary.BreakVector` (`NavMovementComponent.GetVelocityForNavMovement` (`Character.CharacterMovement` _asbp_top_down_character_2))))
        (`Character.LaunchCharacter` _asbp_top_down_character_2 (`KismetMathLibrary.MakeVector` (* _returnvalue_x -4.0) (* _returnvalue_y -4.0)) true false))
      (:`CastFailed`
        (`KismetSystemLibrary.PrintString` "Erreur de jsp")))))

(fn `UserConstructionScript`)