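; BP_TempBridge is a trap bridge that temporarily disappears after something overlaps its trigger Box.
; After a short delay, the Cube loses collision and turns invisible, then returns to solid and visible after a longer wait.
; An IsProcessing flag ignores further overlaps until the cycle finishes.
; The overlap does not filter by actor, so any overlapping component can start it.
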(event `self.ReceiveBeginPlay`)

(event `self.Box.OnComponentBeginOverlap`
  (params (OverlappedComponent :type "PrimitiveComponent Object Reference") (OtherActor :type "Actor Object Reference") (OtherComp :type "PrimitiveComponent Object Reference") (OtherBodyIndex :type Integer) (bFromSweep :type Boolean) (SweepResult :type "HitResult Structure (by ref)"))
  (bind _cube (`self.Cube`))
  (bind _cube_2 (`self.Cube`))
  (if (not (`self.bIsProcessing`))
    (set `self.bIsProcessing` true)
    (`KismetSystemLibrary.Delay` 2.0)
    (`|ExecutionSequence`
      (:`then_0`
        (`PrimitiveComponent.SetCollisionEnabled` _cube_2 "NoCollision"))
      (:`then_1`
        (`SceneComponent.SetVisibility` _cube_2 false false))
      (:`then_2`
        (`KismetSystemLibrary.Delay` 5.0)
        (`|ExecutionSequence`
          (:`then_0`
            (`PrimitiveComponent.SetCollisionEnabled` _cube "QueryAndPhysics"))
          (:`then_1`
            (`SceneComponent.SetVisibility` _cube true false))
          (:`then_2`
            (set `self.bIsProcessing` false)))))))

(fn `UserConstructionScript`)