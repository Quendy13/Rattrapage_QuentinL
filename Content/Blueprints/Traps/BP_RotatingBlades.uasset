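; BP_RotatingBlades is a trap with spinning blades that damages overlapping actors and knocks the player back.
; The looping Tourner timeline, restarted through Retourne, sets Blade1's relative rotation, scaled per axis by Roll, Pitch and Yaw variables.
; DamageCollision overlaps damage the other actor, then launch player 0's BP_TopDownCharacter opposite its horizontal movement velocity, whichever actor overlapped.
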(event `self.ReceiveBeginPlay`
  (bind (_direction _tourne) (`Timeline|Tourner` :!label _label)
    (:`Update`
      (`SceneComponent.K2_SetRelativeRotation` (`self.Blade1`) (`KismetMathLibrary.MakeRotator` (* _tourne (`self.Roll`)) (* _tourne (`self.Pitch`)) (* _tourne (`self.Yaw`))) false false))
    (:`Finished`
      (`self.Retourne`))))

(event `Retourne`
  (goto _label :!via `PlayFromStart`))

(event `self.ReceiveTick`
  (params (DeltaSeconds :type "Float (single-precision)")))

(event `self.DamageCollision.OnComponentBeginOverlap`
  (params (OverlappedComponent :type "PrimitiveComponent Object Reference") (OtherActor :type "Actor Object Reference") (OtherComp :type "PrimitiveComponent Object Reference") (OtherBodyIndex :type Integer) (bFromSweep :type Boolean) (SweepResult :type "HitResult Structure (by ref)"))
  (`GameplayStatics.ApplyDamage` OtherActor 1.0)
  (bind _asbp_top_down_character (cast `/Game/Blueprints/Character/BP_TopDownCharacter` (`GameplayStatics.GetPlayerCharacter` 0))
    (:`then`
      (bind (_returnvalue_x _returnvalue_y) (`KismetMathLibrary.BreakVector` (`NavMovementComponent.GetVelocityForNavMovement` (`Character.CharacterMovement` _asbp_top_down_character))))
      (`Character.LaunchCharacter` _asbp_top_down_character (`KismetMathLibrary.MakeVector` (* _returnvalue_x -4.0) (* _returnvalue_y -4.0)) false false))
    (:`CastFailed`
      (`KismetSystemLibrary.PrintString` "Erreur de jsp"))))

(fn `UserConstructionScript`)