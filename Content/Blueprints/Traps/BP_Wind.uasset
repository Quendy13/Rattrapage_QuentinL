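; BP_Wind is a trap that pushes the top-down player character while it stands inside a wind volume.
; Begin and end overlaps on the Wind component toggle a PlayerInWind flag for BP_TopDownCharacter actors.
; While the flag is set, Tick launches player 0 along the Wall component's right vector scaled by Strength, adding to existing velocity rather than overriding it.
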(event `self.ReceiveBeginPlay`)

(event `self.ReceiveActorBeginOverlap`
  (params (OtherActor :type "Actor Object Reference")))

(event `self.ReceiveTick`
  (params (DeltaSeconds :type "Float (single-precision)"))
  (if (`self.bPlayerInWind`)
    (bind _asbp_top_down_character (cast `/Game/Blueprints/Character/BP_TopDownCharacter` (`GameplayStatics.GetPlayerCharacter` 0)))
    (`Character.LaunchCharacter` _asbp_top_down_character (* (`SceneComponent.GetRightVector` (`self.Wall`)) (`self.Strength`)) false false)))

(event `self.Wind.OnComponentBeginOverlap`
  (params (OverlappedComponent :type "PrimitiveComponent Object Reference") (OtherActor :type "Actor Object Reference") (OtherComp :type "PrimitiveComponent Object Reference") (OtherBodyIndex :type Integer) (bFromSweep :type Boolean) (SweepResult :type "HitResult Structure (by ref)"))
  (cast `/Game/Blueprints/Character/BP_TopDownCharacter` OtherActor)
  (set `self.bPlayerInWind` true))

(event `self.Wind.OnComponentEndOverlap`
  (params (OverlappedComponent :type "PrimitiveComponent Object Reference") (OtherActor :type "Actor Object Reference") (OtherComp :type "PrimitiveComponent Object Reference") (OtherBodyIndex :type Integer))
  (cast `/Game/Blueprints/Character/BP_TopDownCharacter` OtherActor)
  (set `self.bPlayerInWind` false))

(fn `UserConstructionScript`)